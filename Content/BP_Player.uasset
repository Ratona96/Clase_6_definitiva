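; Player character Blueprint that handles Enhanced Input movement, camera look, running and a melee attack.
; Move follows control yaw, and Run switches max walk speed until released.
; Attack, gated by CanAttack, plays a montage chosen by AttackIndex and immediately sphere-traces forward for pawns, sending damage through RecibirDano.
; AttackIndex updates and the socket-based hit trace are disconnected, so the combo never advances.
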(event `self.ReceiveBeginPlay`
  (bind _returnvalue (`InputDeviceLibrary.GetPlayerControllerFromInputDevice` (struct)))
  (`EnhancedInputSubsystemInterface.AddMappingContext` (pcsubsystem `EnhancedInputLocalPlayerSubsystem` _returnvalue) "/Game/IMC_Player.IMC_Player" 0 (struct)))

(event `EnhancedInput|/Game/IA_Move`
  (params (ActionValue :type "Vector2D Structure") (ElapsedSeconds :type "Float (double-precision)") (TriggeredSeconds :type "Float (double-precision)") (InputAction :type "InputAction Object Reference" :default "/Game/IA_Move.IA_Move"))
  (bind (_x _y) (`KismetMathLibrary.BreakVector2D` ActionValue))
  (bind (_returnvalue_roll _returnvalue_pitch _returnvalue_yaw) (`KismetMathLibrary.BreakRotator` (`self.GetControlRotation`)))
  (:`Triggered`
    (`self.AddMovementInput` (`KismetMathLibrary.GetForwardVector` (`KismetMathLibrary.MakeRotator` 0.0 0.0 _returnvalue_yaw)) _y)
    (`self.AddMovementInput` (`KismetMathLibrary.GetRightVector` (`KismetMathLibrary.MakeRotator` 0.0 0.0 _returnvalue_yaw)) _x)))

(event `EnhancedInput|/Game/IA_Look`
  (params (ActionValue :type "Vector2D Structure") (ElapsedSeconds :type "Float (double-precision)") (TriggeredSeconds :type "Float (double-precision)") (InputAction :type "InputAction Object Reference" :default "/Game/IA_Look.IA_Look"))
  (bind (_x _y) (`KismetMathLibrary.BreakVector2D` ActionValue))
  (:`Triggered`
    (`self.AddControllerYawInput` _x)
    (`self.AddControllerPitchInput` _y)))

(event `EnhancedInput|/Game/IA_Run`
  (params (ActionValue :type Boolean) (ElapsedSeconds :type "Float (double-precision)") (TriggeredSeconds :type "Float (double-precision)") (InputAction :type "InputAction Object Reference" :default "/Game/IA_Run.IA_Run"))
  (bind _charactermovement (`self.CharacterMovement`))
  (:`Triggered`
    (set `CharacterMovementComponent.MaxWalkSpeed` 1000.0 _charactermovement))
  (:`Canceled`
    (set `CharacterMovementComponent.MaxWalkSpeed` 400.0 _charactermovement :!label _label))
  (:`Completed`
    (goto _label)))

(event `EnhancedInput|/Game/IA_Attack`
  (params (ActionValue :type Boolean) (ElapsedSeconds :type "Float (double-precision)") (TriggeredSeconds :type "Float (double-precision)") (InputAction :type "InputAction Object Reference" :default "/Game/IA_Attack.IA_Attack"))
  (bind _returnvalue (`self.K2_GetActorLocation`))
  (:`Triggered`
    (`self.CanAttack`
      (:`then`
        (set `self.CanAttack` false)
        (`|PlayMontage` (`self.Mesh`) (select `int` (`self.AttackIndex`) :`0` "/Game/Attacks/01_Montage.01_Montage" :`1` "/Game/Attacks/02_Montage.02_Montage" :`2` "/Game/Attacks/03_Montage.03_Montage" :!type "AnimMontage Object Reference")
          (:`then`
            (bind _outhit (`KismetSystemLibrary.SphereTraceSingleForObjects` _returnvalue (+ (* (`self.GetActorForwardVector`) (200.0 200.0 200.0)) _returnvalue) 0.0 (`|MakeArray` "ObjectTypeQuery3" :!type "EObjectTypeQuery Enum")))
            (message `/Game/BPI_damage.RecibirDano` (`.HitActor` (`GameplayStatics.BreakHitResult` _outhit)) 25.0))
          (:`OnCompleted`
            (set `self.CanAttack` true))))
      (:`else`))))

(fn `UserConstructionScript`)